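; BP_Music is the game's background music actor, looping a three-song playlist from BeginPlay using fixed delays between tracks.
; Its construction script caches the first BP_Menu actor, whose IsGameMuted flag is checked before the second and third songs start.
; AudioisPressed zeroes the playing song's volume multiplier when muted, otherwise restores all three to a boosted level.
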(event Custom|Audio%20is%20Pressed
  ;[1 1 1] Check Which Song is Playing and Mute/Umute
  (if (Variables|/Game/RadialImpact/BluePrints/BP_Menu.BP_Menu_C|GetbIsGameMuted (Variables|ExternalReferences|GetMain%20Menu%20Reference))
    (if (Audio|Components|Audio|IsPlaying (Variables|ObjectVariables|GetSong%2001))
      (Audio|Components|Audio|SetVolumeMultiplier (Variables|ObjectVariables|GetSong%2001) 0.0 :!class /Script/Engine.AudioComponent)
      (elif (Audio|Components|Audio|IsPlaying (Variables|ObjectVariables|GetSong%2002))
        (Audio|Components|Audio|SetVolumeMultiplier (Variables|ObjectVariables|GetSong%2002) 0.0 :!class /Script/Engine.AudioComponent)
        (elif (Audio|Components|Audio|IsPlaying (Variables|ObjectVariables|GetSong%2003))
          (Audio|Components|Audio|SetVolumeMultiplier (Variables|ObjectVariables|GetSong%2003) 0.0 :!class /Script/Engine.AudioComponent))))
    (else
      (Audio|Components|Audio|SetVolumeMultiplier (Variables|ObjectVariables|GetSong%2002) 1.5 :!class /Script/Engine.AudioComponent))))

(event EventBeginPlay
  ;[1 1 1] Song Loop Playlist
  (Audio|Components|Audio|Play (Variables|ObjectVariables|GetSong%2001) 0.0 :!label _label)
  (Utilities|FlowControl|Delay 289.0)
  (if (Variables|/Game/RadialImpact/BluePrints/BP_Menu.BP_Menu_C|GetbIsGameMuted (Variables|ExternalReferences|GetMain%20Menu%20Reference))
    (Audio|Components|Audio|SetVolumeMultiplier (Variables|ObjectVariables|GetSong%2002) 0.0 :!class /Script/Engine.AudioComponent))
  (Audio|Components|Audio|Play (Variables|ObjectVariables|GetSong%2002) 0.0)
  (Utilities|FlowControl|Delay 208.0)
  (if (Variables|/Game/RadialImpact/BluePrints/BP_Menu.BP_Menu_C|GetbIsGameMuted (Variables|ExternalReferences|GetMain%20Menu%20Reference))
    (Audio|Components|Audio|SetVolumeMultiplier (Variables|ObjectVariables|GetSong%2003) 0.0 :!class /Script/Engine.AudioComponent))
  (Audio|Components|Audio|Play (Variables|ObjectVariables|GetSong%2003) 0.0)
  (Utilities|FlowControl|Delay 291.0)
  (goto _label))

(fn ConstructionScript
  (bind _outactors (Actor|GetAllActorsOfClass "/Game/RadialImpact/BluePrints/BP_Menu.BP_Menu_C"))
  (Variables|ExternalReferences|SetMain%20Menu%20Reference (Utilities|Array|Get(acopy) _outactors)))