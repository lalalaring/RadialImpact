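; Animated space backdrop actor with three star layers and randomly rotated nebula layers.
; The construction script creates a dynamic material instance per star layer and randomizes four nebula pitches; BeginPlay re-randomizes all but the far-back one.
; Each star layer uses timelines to lerp "Star Color" toward random colors and loop a "Star Intensity" curve.
; Delays fired from color timeline updates restart the cycles at different intervals per layer.
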(event Custom|Animate%20Star%20Background%2003
  ;[1 1 1] Animates Back Background
  (Utilities|FlowControl|Sequence
    (:then_0
      (bind _returnvalue (Rendering|Material|GetVectorParameterValue (Variables|MaterialInstances|GetStar%20Background%2003%20MI) "Star Color" :!class /Script/Engine.MaterialInstanceDynamic :!label _label))
      (Variables|ColorVariables|SetThird%20Color (Math|Color|MakeColor (Math|Random|RandomFloat) (Math|Random|RandomFloat) (Math|Random|RandomFloat)))
      (bind _star_color_curve (Timeline|Star%20Color%20Animation%2003 PlayFromStart)
        (:Update
          (Rendering|Material|SetVectorParameterValue (Variables|MaterialInstances|GetStar%20Background%2003%20MI) "Star Color" (Math|Color|Lerp(LinearColor) _returnvalue (Variables|ColorVariables|GetThird%20Color) _star_color_curve) :!class /Script/Engine.MaterialInstanceDynamic)
          (Utilities|FlowControl|Delay 7.0)
          (Utilities|FlowControl|Sequence
            (:then_0
              (goto _label))
            (:then_1
              _)))))
    (:then_1
      _))
  (Rendering|Material|GetScalarParameterValue (Variables|MaterialInstances|GetStar%20Background%2003%20MI) "Star Intensity" :!class /Script/Engine.MaterialInstanceDynamic :!label _label_2)
  (bind _star_intensity_curve (Timeline|Star%20Intensity%2003 PlayFromStart)
    (:Update
      (Rendering|Material|SetScalarParameterValue (Variables|MaterialInstances|GetStar%20Background%2003%20MI) "Star Intensity" _star_intensity_curve :!class /Script/Engine.MaterialInstanceDynamic))
    (:Finished
      (goto _label_2))))

(event Custom|Animate%20Star%20Background%2001
  ;[1 1 1] Animates the Star Background
  (Utilities|FlowControl|Sequence
    (:then_0
      (bind _returnvalue (Rendering|Material|GetVectorParameterValue (Variables|MaterialInstances|GetBackground%20MI) "Star Color" :!class /Script/Engine.MaterialInstanceDynamic :!label _label))
      ;;[0.9733 0.01116 1] Animates the Color Change for Stars
      (Variables|ColorVariables|SetNew%20Color (Math|Color|MakeColor (Math|Random|RandomFloat) (Math|Random|RandomFloat) (Math|Random|RandomFloat)))
      (bind _star_color_curve (Timeline|Star%20Animation%20Curves PlayFromStart)
        (:Update
          (Rendering|Material|SetVectorParameterValue (Variables|MaterialInstances|GetBackground%20MI) "Star Color" (Math|Color|Lerp(LinearColor) _returnvalue (Variables|ColorVariables|GetNew%20Color) _star_color_curve) :!class /Script/Engine.MaterialInstanceDynamic)
          (Utilities|FlowControl|Delay 5.0)
          (Utilities|FlowControl|Sequence
            (:then_0
              (goto _label))
            (:then_1
              _)))))
    (:then_1
      _))
  ;;[0.7929 0.003757 1] Animates the Color Intensity of the Stars
  (Rendering|Material|GetScalarParameterValue (Variables|MaterialInstances|GetBackground%20MI) "Star Intensity" :!class /Script/Engine.MaterialInstanceDynamic :!label _label_2)
  (bind _star_intensity_curve (Timeline|Star%20Intensity%20Animation PlayFromStart)
    (:Update
      (Rendering|Material|SetScalarParameterValue (Variables|MaterialInstances|GetBackground%20MI) "Star Intensity" _star_intensity_curve :!class /Script/Engine.MaterialInstanceDynamic))
    (:Finished
      (goto _label_2))))

(event Custom|Animate%20Star%20Background%2002
  ;[1 1 1] Animates Middle Background
  (Utilities|FlowControl|Sequence
    (:then_0
      (bind _returnvalue (Rendering|Material|GetVectorParameterValue (Variables|MaterialInstances|GetStar%20Background%2002%20MI) "Star Color" :!class /Script/Engine.MaterialInstanceDynamic :!label _label))
      (Variables|ColorVariables|SetSecond%20Color (Math|Color|MakeColor (Math|Random|RandomFloat) (Math|Random|RandomFloat) (Math|Random|RandomFloat)))
      (bind _star_color_curve (Timeline|Star%20Color%20Animation%2002 PlayFromStart)
        (:Update
          (Rendering|Material|SetVectorParameterValue (Variables|MaterialInstances|GetStar%20Background%2002%20MI) "Star Color" (Math|Color|Lerp(LinearColor) _returnvalue (Variables|ColorVariables|GetSecond%20Color) _star_color_curve) :!class /Script/Engine.MaterialInstanceDynamic)
          (Utilities|FlowControl|Delay 3.0)
          (Utilities|FlowControl|Sequence
            (:then_0
              (goto _label))
            (:then_1
              _)))))
    (:then_1
      _))
  (Rendering|Material|GetScalarParameterValue (Variables|MaterialInstances|GetStar%20Background%2002%20MI) "Star Intensity" :!class /Script/Engine.MaterialInstanceDynamic :!label _label_2)
  (bind _star_intensity_curve (Timeline|Star%20Intensity%2002 PlayFromStart)
    (:Update
      (Rendering|Material|SetScalarParameterValue (Variables|MaterialInstances|GetStar%20Background%2002%20MI) "Star Intensity" _star_intensity_curve :!class /Script/Engine.MaterialInstanceDynamic))
    (:Finished
      (goto _label_2))))

(event EventBeginPlay
  ;[1 1 1] Animates the Star Background
  (Transformation|SetWorldRotation (Variables|ObjectVariables|GetNebula_Front) (Class|KismetMathLibrary|MakeRot (Math|Random|RandomFloatinRange -89.0 89.0) 0.0 -9e+01) false)
  (Transformation|SetWorldRotation (Variables|ObjectVariables|GetNebula_Middle) (Class|KismetMathLibrary|MakeRot (Math|Random|RandomFloatinRange -89.0 89.0) 0.0 -9e+01) false)
  (Transformation|SetWorldRotation (Variables|ObjectVariables|GetNebula_Back) (Class|KismetMathLibrary|MakeRot (Math|Random|RandomFloatinRange -89.0 89.0) 0.0 -9e+01) false)
  (CallFunction|AnimateStarBackground01)
  (CallFunction|AnimateStarBackground02)
  (CallFunction|AnimateStarBackground03))

(fn ConstructionScript
  (bind _returnvalue (Rendering|Material|CreateDynamicMaterialInstance (Variables|ObjectVariables|GetStar%20Background) 0 0 :!class /Script/Engine.PrimitiveComponent))
  (Variables|MaterialInstances|SetBackground%20MI _returnvalue)
  (Transformation|SetWorldRotation (Variables|ObjectVariables|GetNebula_Front) (Class|KismetMathLibrary|MakeRot (Math|Random|RandomFloatinRange -89.0 89.0) 0.0 -9e+01) false)
  (Transformation|SetWorldRotation (Variables|ObjectVariables|GetNebula_Middle) (Class|KismetMathLibrary|MakeRot (Math|Random|RandomFloatinRange -89.0 89.0) 0.0 -9e+01) false)
  (Transformation|SetWorldRotation (Variables|ObjectVariables|GetNebula_Back) (Class|KismetMathLibrary|MakeRot (Math|Random|RandomFloatinRange -89.0 89.0) 0.0 -9e+01) false)
  (Transformation|SetWorldRotation (Variables|ObjectVariables|GetNebula_FarBack) (Class|KismetMathLibrary|MakeRot (Math|Random|RandomFloatinRange -89.0 89.0) 0.0 -9e+01) false)
  (bind _returnvalue_2 (Rendering|Material|CreateDynamicMaterialInstance (Variables|ObjectVariables|GetStar%20Background%2002) 0 0 :!class /Script/Engine.PrimitiveComponent))
  (Variables|MaterialInstances|SetStar%20Background%2002%20MI _returnvalue_2)
  (bind _returnvalue_3 (Rendering|Material|CreateDynamicMaterialInstance (Variables|ObjectVariables|GetStar%20Background%2003) 0 0 :!class /Script/Engine.PrimitiveComponent))
  (Variables|MaterialInstances|SetStar%20Background%2003%20MI _returnvalue_3))