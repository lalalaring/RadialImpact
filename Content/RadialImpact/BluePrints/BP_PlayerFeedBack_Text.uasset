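; Player feedback text actor with hit-rating labels from Miss to Perfect and unlock notices for the 10, 25 and 50 wave modes.
; Construction creates dynamic materials for every label and hides the unlock notices, while BeginPlay hides the ratings, which are not animated here.
; Each unlock event shows its notice, fades opacity through a timeline, then uses Delays chained off Update to reverse the fade and hide it.
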(event Custom|Animate%2050%20Waves%20Unlock
  ;[1 1 1] Show the 50 Waves Mode Unlocked Text
  (Rendering|SetVisibility (Variables|ObjectVariables|Get50%20Waves%20Unlocked) true false)
  (Rendering|Material|SetScalarParameterValue (Variables|MaterialInstances|Get50%20Waves%20Unlocked%20MI) "Opacity" 0.0 :!class /Script/Engine.MaterialInstanceDynamic)
  (Utilities|FlowControl|Delay 0.2)
  (bind _color_curve (Timeline|50%20Waves%20Unlocked%20Animation PlayFromStart)
    (:Update
      (Rendering|Material|SetScalarParameterValue (Variables|MaterialInstances|Get50%20Waves%20Unlocked%20MI) "Opacity" (Math|Float|Lerp 0.0 1.0 _color_curve) :!class /Script/Engine.MaterialInstanceDynamic)
      (Utilities|FlowControl|Delay 3.0)
      (Components|Timeline|ReversefromEnd (Variables|Default|Get50%20Waves%20Unlocked%20Animation))
      (Utilities|FlowControl|Delay 1.0)
      (Rendering|SetVisibility (Variables|ObjectVariables|Get50%20Waves%20Unlocked) false false))))

(event Custom|Animate%2010%20Waves%20Unlocked
  ;[1 1 1] Show the 10 Waves Mode Unlocked Text
  (Rendering|SetVisibility (Variables|ObjectVariables|Get10%20Waves%20Unlocked) true false)
  (Rendering|Material|SetScalarParameterValue (Variables|MaterialInstances|Get10%20Waves%20Unlocked%20MI) "Opacity" 0.0 :!class /Script/Engine.MaterialInstanceDynamic)
  (Utilities|FlowControl|Delay 0.2)
  (bind _color_curve (Timeline|10%20Waves%20Unlocked%20Animation PlayFromStart)
    (:Update
      (Rendering|Material|SetScalarParameterValue (Variables|MaterialInstances|Get10%20Waves%20Unlocked%20MI) "Opacity" (Math|Float|Lerp 0.0 1.0 _color_curve) :!class /Script/Engine.MaterialInstanceDynamic)
      (Utilities|FlowControl|Delay 3.0)
      (Components|Timeline|ReversefromEnd (Variables|Default|Get10%20Waves%20Unlocked%20Animation))
      (Utilities|FlowControl|Delay 1.0)
      (Rendering|SetVisibility (Variables|ObjectVariables|Get10%20Waves%20Unlocked) false false))))

(event Custom|Animate%2025%20Waves%20Unlock
  ;[1 1 1] Show the 25 Waves Mode Unlocked Text
  (Rendering|SetVisibility (Variables|ObjectVariables|Get25%20Waves%20Unlocked) true false)
  (Rendering|Material|SetScalarParameterValue (Variables|MaterialInstances|Get25%20Waves%20Unlocked%20MI) "Opacity" 0.0 :!class /Script/Engine.MaterialInstanceDynamic)
  (Utilities|FlowControl|Delay 0.2)
  (bind _color_curve (Timeline|25%20Waves%20Unlocked%20Animation PlayFromStart)
    (:Update
      (Rendering|Material|SetScalarParameterValue (Variables|MaterialInstances|Get25%20Waves%20Unlocked%20MI) "Opacity" (Math|Float|Lerp 0.0 1.0 _color_curve) :!class /Script/Engine.MaterialInstanceDynamic)
      (Utilities|FlowControl|Delay 3.0)
      (Components|Timeline|ReversefromEnd (Variables|Default|Get25%20Waves%20Unlocked%20Animation))
      (Utilities|FlowControl|Delay 1.0)
      (Rendering|SetVisibility (Variables|ObjectVariables|Get25%20Waves%20Unlocked) false false))))

(event EventBeginPlay
  ;[1 1 1] Sets Initial Visibility of Feedback Text
  (Rendering|SetVisibility (Variables|ObjectVariables|GetMiss) false false))

(fn ConstructionScript
  (bind _returnvalue (Rendering|Material|CreateDynamicMaterialInstance (Variables|ObjectVariables|GetPerfect) 0 0 :!class /Script/Engine.PrimitiveComponent))
  (Variables|MaterialInstances|SetPerfect%20Text%20MI _returnvalue)
  (bind _returnvalue_2 (Rendering|Material|CreateDynamicMaterialInstance (Variables|ObjectVariables|GetExcellent) 0 0 :!class /Script/Engine.PrimitiveComponent))
  (Variables|MaterialInstances|SetExcellent%20Text%20MI _returnvalue_2)
  (bind _returnvalue_3 (Rendering|Material|CreateDynamicMaterialInstance (Variables|ObjectVariables|GetGood) 0 0 :!class /Script/Engine.PrimitiveComponent))
  (Variables|MaterialInstances|SetGood%20Text%20MI _returnvalue_3)
  (bind _returnvalue_4 (Rendering|Material|CreateDynamicMaterialInstance (Variables|ObjectVariables|GetOK) 0 0 :!class /Script/Engine.PrimitiveComponent))
  (Variables|MaterialInstances|SetOK%20Text%20MI _returnvalue_4)
  (bind _returnvalue_5 (Rendering|Material|CreateDynamicMaterialInstance (Variables|ObjectVariables|GetBad) 0 0 :!class /Script/Engine.PrimitiveComponent))
  (Variables|MaterialInstances|SetBad%20Text%20MI _returnvalue_5)
  (bind _returnvalue_6 (Rendering|Material|CreateDynamicMaterialInstance (Variables|ObjectVariables|GetMiss) 0 0 :!class /Script/Engine.PrimitiveComponent))
  (Variables|MaterialInstances|SetMiss%20Text%20MI _returnvalue_6)
  (Rendering|SetVisibility (Variables|ObjectVariables|Get10%20Waves%20Unlocked) false false)
  (bind _returnvalue_7 (Rendering|Material|CreateDynamicMaterialInstance (Variables|ObjectVariables|Get10%20Waves%20Unlocked) 0 0 :!class /Script/Engine.PrimitiveComponent))
  (Variables|MaterialInstances|Set10%20Waves%20Unlocked%20MI _returnvalue_7)
  (Rendering|SetVisibility (Variables|ObjectVariables|Get25%20Waves%20Unlocked) false false)
  (bind _returnvalue_8 (Rendering|Material|CreateDynamicMaterialInstance (Variables|ObjectVariables|Get25%20Waves%20Unlocked) 0 0 :!class /Script/Engine.PrimitiveComponent))
  (Variables|MaterialInstances|Set25%20Waves%20Unlocked%20MI _returnvalue_8)
  (Rendering|SetVisibility (Variables|ObjectVariables|Get50%20Waves%20Unlocked) false false)
  (bind _returnvalue_9 (Rendering|Material|CreateDynamicMaterialInstance (Variables|ObjectVariables|Get50%20Waves%20Unlocked) 0 0 :!class /Script/Engine.PrimitiveComponent))
  (Variables|MaterialInstances|Set50%20Waves%20Unlocked%20MI _returnvalue_9))