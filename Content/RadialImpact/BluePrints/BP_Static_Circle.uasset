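; Static target circle that pairs with BP_Dynamic_Circle and forwards its click and touch input to it.
; BeginPlay randomizes a red, green or blue-dominant tint through a dynamic material instance, randomizes scale, then calls SetDynamicCircle on its partner.
; ChangeColor repeats this after ChangeLocation, which moves both circles to a random XZ point, or a fixed one during menus or wave selection.
; The construction script caches partner, menu and game mode references.
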(event OnInputTouchBegin(StaticCircle)
  (params (FingerIndex :type ETouchIndex%20Enum :default "Touch1") (TouchedComponent :type Primitive%20Component%20Object%20Reference))
  ;[1 1 1] Static Circle Input Calls
  (Default|StaticCircleTouched (Variables|ExternalReferences|GetDynamic%20Circle%20Reference)))

(event OnClicked(StaticCircle)
  (params (TouchedComponent :type Primitive%20Component%20Object%20Reference))
  ;[1 1 1] Static Circle Input Calls
  (Default|StaticCircleClicked (Variables|ExternalReferences|GetDynamic%20Circle%20Reference)))

(event Custom|Change%20Color
  (bind _returnvalue (Math|Random|RandomIntegerinRange 0 2))
  (bind _smallest_static_circle (Variables|FloatVariables|GetSmallest%20Static%20Circle))
  (bind _largest_static_circle (Variables|FloatVariables|GetLargest%20Static%20Circle))
  (bind _default_size (Variables|VectorVariables|GetDefault%20Size))
  (bind _returnvalue_2 (* _default_size _largest_static_circle))
  (bind _returnvalue_3 (* _default_size _smallest_static_circle))
  (bind _x (Math|Vector|BreakVector _returnvalue_3))
  (bind _x_2 (Math|Vector|BreakVector _returnvalue_2))
  (bind _returnvalue_4 (Math|Random|RandomFloatinRange _x _x_2))
  (CallFunction|ChangeLocation)
  (if (== _returnvalue 0) :!label _label
    ;[1 1 1] Set Scale of Static Circle
    (Rendering|Material|SetVectorParameterValue (Variables|MaterialInstances|GetStatic%20Circle%20MI) "Static Circle Color" (Math|Color|MakeColor (Math|Random|RandomFloatinRange 1.0 1.0) (Math|Random|RandomFloatinRange 0.3 0.5) (Math|Random|RandomFloatinRange 0.3 0.5) 1.0) :!class /Script/Engine.MaterialInstanceDynamic)
    (elif (== _returnvalue 1)
      ;[1 1 1] Randomizes the Color of the Static Circle
      (Rendering|Material|SetVectorParameterValue (Variables|MaterialInstances|GetStatic%20Circle%20MI) "Static Circle Color" (Math|Color|MakeColor (Math|Random|RandomFloatinRange 0.3 0.5) (Math|Random|RandomFloatinRange 1.0 1.0) (Math|Random|RandomFloatinRange 0.3 0.5) 1.0) :!class /Script/Engine.MaterialInstanceDynamic)
      (elif (== _returnvalue 2)
        (Rendering|Material|SetVectorParameterValue (Variables|MaterialInstances|GetStatic%20Circle%20MI) "Static Circle Color" (Math|Color|MakeColor (Math|Random|RandomFloatinRange 0.3 0.5) (Math|Random|RandomFloatinRange 0.3 0.5) (Math|Random|RandomFloatinRange 1.0 1.0) 1.0) :!class /Script/Engine.MaterialInstanceDynamic)
        (else
          (goto _label)))))
  (Transformation|SetWorldScale3D (Variables|ObjectVariables|GetStatic%20Circle) (Math|Vector|MakeVector _returnvalue_4 _returnvalue_4 _returnvalue_4))
  (Default|SetDynamicCircle (Variables|ExternalReferences|GetDynamic%20Circle%20Reference)))

(event Custom|Change%20Location
  ;[1 1 1] Randomizes the Location of the Circles if Not in any Menus
  (if (Variables|/Game/RadialImpact/BluePrints/BP_Menu.BP_Menu_C|GetbisOnMenu (Variables|ExternalReferences|GetMain%20Menu%20Reference))
    (Transformation|SetWorldLocation (Variables|ObjectVariables|GetStatic%20Circle) "1250.000000, 0,760.000000" false false :!label _label)
    (Transformation|SetWorldLocation (Variables|/Game/RadialImpact/BluePrints/BP_Dynamic_Circle.BP_Dynamic_Circle_C|GetDynamic%20Circle (Variables|ExternalReferences|GetDynamic%20Circle%20Reference)) "1250.000000, 0,760.000000" false false)
    (elif (Variables|/Game/RadialImpact/BluePrints/BP_GameMode_Actor.BP_GameMode_Actor_C|GetbSelectingWavesOptions (Variables|ExternalReferences|GetGame%20Mode%20Reference))
      (goto _label)
      (else
        (Variables|VectorVariables|SetNew%20Location (Math|Vector|MakeVector (Math|Random|RandomFloatinRange 8.6e+02 1.6e+03) 0.0 (Math|Random|RandomFloatinRange 5.6e+02 9.6e+02)))
        (Transformation|SetWorldLocation (Variables|ObjectVariables|GetStatic%20Circle) (Variables|VectorVariables|GetNew%20Location) false false)
        (Transformation|SetWorldLocation (Variables|/Game/RadialImpact/BluePrints/BP_Dynamic_Circle.BP_Dynamic_Circle_C|GetDynamic%20Circle (Variables|ExternalReferences|GetDynamic%20Circle%20Reference)) (Variables|VectorVariables|GetNew%20Location) false false)))))

(event EventBeginPlay
  (bind _returnvalue (Math|Random|RandomIntegerinRange 0 2))
  (bind _smallest_static_circle (Variables|FloatVariables|GetSmallest%20Static%20Circle))
  (bind _largest_static_circle (Variables|FloatVariables|GetLargest%20Static%20Circle))
  (bind _default_size (Variables|VectorVariables|GetDefault%20Size))
  (bind _returnvalue_2 (* _default_size _largest_static_circle))
  (bind _returnvalue_3 (* _default_size _smallest_static_circle))
  (bind _x (Math|Vector|BreakVector _returnvalue_3))
  (bind _x_2 (Math|Vector|BreakVector _returnvalue_2))
  (bind _returnvalue_4 (Math|Random|RandomFloatinRange _x _x_2))
  (if (== _returnvalue 0) :!label _label
    ;[1 1 1] Set Scale of Static Circle
    (Rendering|Material|SetVectorParameterValue (Variables|MaterialInstances|GetStatic%20Circle%20MI) "Static Circle Color" (Math|Color|MakeColor (Math|Random|RandomFloatinRange 1.0 1.0) (Math|Random|RandomFloatinRange 0.3 0.5) (Math|Random|RandomFloatinRange 0.3 0.5) 1.0) :!class /Script/Engine.MaterialInstanceDynamic)
    (elif (== _returnvalue 1)
      ;[1 1 1] Randomizes the Color of the Static Circle
      (Rendering|Material|SetVectorParameterValue (Variables|MaterialInstances|GetStatic%20Circle%20MI) "Static Circle Color" (Math|Color|MakeColor (Math|Random|RandomFloatinRange 0.3 0.5) (Math|Random|RandomFloatinRange 1.0 1.0) (Math|Random|RandomFloatinRange 0.3 0.5) 1.0) :!class /Script/Engine.MaterialInstanceDynamic)
      (elif (== _returnvalue 2)
        (Rendering|Material|SetVectorParameterValue (Variables|MaterialInstances|GetStatic%20Circle%20MI) "Static Circle Color" (Math|Color|MakeColor (Math|Random|RandomFloatinRange 0.3 0.5) (Math|Random|RandomFloatinRange 0.3 0.5) (Math|Random|RandomFloatinRange 1.0 1.0) 1.0) :!class /Script/Engine.MaterialInstanceDynamic)
        (else
          (goto _label)))))
  (Transformation|SetWorldScale3D (Variables|ObjectVariables|GetStatic%20Circle) (Math|Vector|MakeVector _returnvalue_4 _returnvalue_4 _returnvalue_4))
  (Default|SetDynamicCircle (Variables|ExternalReferences|GetDynamic%20Circle%20Reference)))

(fn ConstructionScript
  (bind _returnvalue (Rendering|Material|CreateDynamicMaterialInstance (Variables|ObjectVariables|GetStatic%20Circle) 0 "/Game/RadialImpact/Materials/Circles/MAT_Static_Circle.MAT_Static_Circle" :!class /Script/Engine.PrimitiveComponent))
  (Variables|MaterialInstances|SetStatic%20Circle%20MI _returnvalue)
  (bind _outactors (Actor|GetAllActorsOfClass "/Game/RadialImpact/BluePrints/BP_Dynamic_Circle.BP_Dynamic_Circle_C"))
  (Variables|ExternalReferences|SetDynamic%20Circle%20Reference (Utilities|Array|Get(acopy) _outactors))
  (Variables|VectorVariables|SetDefault%20Size (Variables|/Script/Engine.SceneComponent|GetRelativeScale3D (Variables|ObjectVariables|GetStatic%20Circle)))
  (bind _outactors_2 (Actor|GetAllActorsOfClass "/Game/RadialImpact/BluePrints/BP_Menu.BP_Menu_C"))
  (Variables|ExternalReferences|SetMain%20Menu%20Reference (Utilities|Array|Get(acopy) _outactors_2))
  (bind _outactors_3 (Actor|GetAllActorsOfClass "/Game/RadialImpact/BluePrints/BP_GameMode_Actor.BP_GameMode_Actor_C"))
  (Variables|ExternalReferences|SetGame%20Mode%20Reference (Utilities|Array|Get(acopy) _outactors_3)))