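; BP_ScoreText is the score feedback display, with components for six hit ratings from Miss to Perfect plus a combo point value.
; The Construction Script gives each component a dynamic material instance and gathers the six ratings into a FeedbackText array.
; BeginPlay hides all values, colors the Miss material red and scales the array to 1.25 times the first element's world scale.
; No logic here reveals or updates them.
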(event EventBeginPlay
  ;[1 1 1] Sets Initial Visibility and Scale of Score Values
  (Rendering|SetVisibility (Variables|ObjectVariables|GetMiss%20Score%20Value) false false)
  (Rendering|Material|SetVectorParameterValue (Variables|MaterialInstances|GetMiss%20Score%20Value%20MI) "Miss Score Text Color" "(R=1.000000,G=0.000000,B=0.000000,A=1.000000)" :!class /Script/Engine.MaterialInstanceDynamic)
  (Transformation|SetRelativeScale3D (Variables|ArrayVariables|GetFeedback%20Text) (* (Transformation|GetWorldScale (Utilities|Array|Get(acopy) (Variables|ArrayVariables|GetFeedback%20Text))) 1.25))
  (Rendering|SetVisibility (Variables|ObjectVariables|GetCombo%20Point%20Value) false false))

(fn ConstructionScript
  (bind _returnvalue (Rendering|Material|CreateDynamicMaterialInstance (Variables|ObjectVariables|GetPerfect%20Score%20Value) 0 0 :!class /Script/Engine.PrimitiveComponent))
  (Variables|MaterialInstances|SetPerfect%20Score%20Value%20MI _returnvalue)
  (bind _returnvalue_2 (Rendering|Material|CreateDynamicMaterialInstance (Variables|ObjectVariables|GetExcellent%20Score%20Value) 0 0 :!class /Script/Engine.PrimitiveComponent))
  (Variables|MaterialInstances|SetExcellent%20Score%20Value%20MI _returnvalue_2)
  (bind _returnvalue_3 (Rendering|Material|CreateDynamicMaterialInstance (Variables|ObjectVariables|GetGood%20Score%20Value) 0 0 :!class /Script/Engine.PrimitiveComponent))
  (Variables|MaterialInstances|SetGood%20Score%20Value%20MI _returnvalue_3)
  (bind _returnvalue_4 (Rendering|Material|CreateDynamicMaterialInstance (Variables|ObjectVariables|GetOK%20Score%20Value) 0 0 :!class /Script/Engine.PrimitiveComponent))
  (Variables|MaterialInstances|SetOK%20Score%20Value%20MI _returnvalue_4)
  (bind _returnvalue_5 (Rendering|Material|CreateDynamicMaterialInstance (Variables|ObjectVariables|GetBad%20Score%20Value) 0 0 :!class /Script/Engine.PrimitiveComponent))
  (Variables|MaterialInstances|SetBad%20Score%20Value%20MI _returnvalue_5)
  (bind _returnvalue_6 (Rendering|Material|CreateDynamicMaterialInstance (Variables|ObjectVariables|GetMiss%20Score%20Value) 0 0 :!class /Script/Engine.PrimitiveComponent))
  (Variables|MaterialInstances|SetMiss%20Score%20Value%20MI _returnvalue_6)
  (Utilities|Array|Add (Variables|ArrayVariables|GetFeedback%20Text) (Variables|ObjectVariables|GetMiss%20Score%20Value))
  (Utilities|Array|Add (Variables|ArrayVariables|GetFeedback%20Text) (Variables|ObjectVariables|GetBad%20Score%20Value))
  (Utilities|Array|Add (Variables|ArrayVariables|GetFeedback%20Text) (Variables|ObjectVariables|GetOK%20Score%20Value))
  (Utilities|Array|Add (Variables|ArrayVariables|GetFeedback%20Text) (Variables|ObjectVariables|GetGood%20Score%20Value))
  (Utilities|Array|Add (Variables|ArrayVariables|GetFeedback%20Text) (Variables|ObjectVariables|GetExcellent%20Score%20Value))
  (Utilities|Array|Add (Variables|ArrayVariables|GetFeedback%20Text) (Variables|ObjectVariables|GetPerfect%20Score%20Value))
  (bind _returnvalue_7 (Rendering|Material|CreateDynamicMaterialInstance (Variables|ObjectVariables|GetCombo%20Point%20Value) 0 0 :!class /Script/Engine.PrimitiveComponent))
  (Variables|MaterialInstances|SetCombo%20Point%20Value%20MI _returnvalue_7))